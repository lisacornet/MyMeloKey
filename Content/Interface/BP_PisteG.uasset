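; Left lane of a rhythm game, spawning notes to the music and judging Left key presses.
; A muted MetaSound copy runs ahead of the delayed audible track, its watched beatmap output spawning NoteGauche actors.
; Tick tracks hitbox overlap; presses flash the arrow and grade note age into score, combo and feedback widgets, or reset combo when no note overlaps.
; The FinG trigger destroys actors reaching the end.
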(event OnComponentBeginOverlap(FinG)
  (params (OverlappedComponent :type Primitive%20Component%20Object%20Reference) (OtherActor :type Actor%20Object%20Reference) (OtherComp :type Primitive%20Component%20Object%20Reference) (OtherBodyIndex :type Integer) (bFromSweep :type Boolean) (SweepResult :type Hit%20Result%20Structure%20%28by%20ref%29))
  (Actor|DestroyActor OtherActor))

(event Custom|SuiviBeatmapG
  (params (OutputName :type Name) (Output :type Meta%20Sound%20Output%20Structure%20%28by%20ref%29))
  (bind _returnvalue (Game|SpawnActorfromClass "/Game/Interface/NoteGauche.NoteGauche_C" (Math|Transform|MakeTransform (Variables|/Script/Engine.SceneComponent|GetRelativeLocation (Variables|Default|GetSpawnerG)) "0, 0, 0" "1.000000,1.000000,1.000000") "Undefined" "MultiplyWithRoot" 0 0))
  (Default|CreationNoteGauche _returnvalue))

(event EventTick
  (params (DeltaSeconds :type Float%20%28single-precision%29))
  (if (== (Utilities|Array|Length (Collision|GetOverlappingActors (Variables|Default|GetHitboxG) "/Game/Interface/NoteGauche.NoteGauche_C" :!class /Script/Engine.PrimitiveComponent)) 0)
    (Variables|Default|SetNoteCollision? false)
    (else
      (Variables|Default|SetNoteCollision? true))))

(event EventBeginPlay
  (Input|EnableInput (Game|GetPlayerController 0))
  (Utilities|FlowControl|Sequence
    (:then_0
      (Utilities|FlowControl|Delay 3.1)
      (AddComponent|AddAudioComponent false))
    (:then_1
      (bind _returnvalue (AddComponent|AddAudioComponent false))
      (MetaSoundOutput|WatchOutput (WorldSubsystems|GetMetaSoundOutputSubsystem) _returnvalue "TheManBeatmapLeft" (delegate Custom|SuiviBeatmapG) "None" "None" :!class /Script/MetasoundEngine.MetaSoundOutputSubsystem)
      (Audio|Components|Audio|SetVolumeMultiplier _returnvalue 0.0 :!class /Script/Engine.AudioComponent))))

(event Input|KeyboardEvents|Left
  (params (Key :type Key%20Structure :default "None"))
  (bind _flecheg (Variables|Default|GetFlecheG))
  (:Pressed
    (Rendering|Material|SetMaterial _flecheg 0 "/Game/Interface/flecheGrisAppuyée_Mat.flecheGrisAppuyée_Mat")
    (Utilities|FlowControl|Delay 0.2)
    (Rendering|Material|SetMaterial _flecheg 0 "/Game/Interface/flecheGris_Mat.flecheGris_Mat")
    (if (Variables|Default|GetNoteCollision?)
      (bind _returnvalue (Actor|GetActorOfClass "/Game/Interface/NoteGauche.NoteGauche_C"))
      (bind _output_get (Variables|Default|SetNoteActuelle _returnvalue))
      (Variables|Default|SetTempsReaction (- (Utilities|Time|GetGameTimeinSeconds) (Variables|/Game/Interface/NoteGauche.NoteGauche_C|GetTempsCreation _output_get)))
      (CallFunction|ResultatTouche)
      (else
        (bind _asjeu (Utilities|Casting|CastToJeu (Game|GetGameMode)))
        (Variables|/Game/Joueur/Jeu.Jeu_C|SetCombo _asjeu 0)
        (bind _returnvalue_2 (UserInterface|CreateWidget "/Game/Interface/FeedbackRate.FeedbackRate_C"))
        (Class|UserWidget|SetDesiredSizeinViewport _returnvalue_2 "(X=210.000000,Y=120.000000)")
        (Class|UserWidget|SetPositioninViewport _returnvalue_2 "(X=640.000000,Y=800.000000)" false)
        (UserInterface|Viewport|AddtoPlayerScreen _returnvalue_2)))))

(fn ConstructionScript)

(fn ResultatTouche
  (bind _tempsreaction (Variables|Default|GetTempsReaction))
  (bind _tempsreaction_2 (Variables|Default|GetTempsReaction))
  (if (and (>= _tempsreaction 3.0) (<= _tempsreaction 3.2))
    (Utilities|FlowControl|Sequence
      (:then_0
        (bind _asjeu (Utilities|Casting|CastToJeu (Game|GetGameMode)))
        (Variables|/Game/Joueur/Jeu.Jeu_C|SetScore _asjeu (+ (Variables|/Game/Joueur/Jeu.Jeu_C|GetScore _asjeu) 250))
        (bind _result (Math|Integer|IncrementInt (Variables|/Game/Joueur/Jeu.Jeu_C|GetCombo _asjeu))
          (:%20%20
            (Variables|/Game/Joueur/Jeu.Jeu_C|SetCombo _asjeu _result))))
      (:then_1
        (bind _returnvalue (UserInterface|CreateWidget "/Game/Interface/FeedbackSuper.FeedbackSuper_C"))
        (Class|UserWidget|SetDesiredSizeinViewport _returnvalue "(X=260.000000,Y=120.000000)")
        (Class|UserWidget|SetPositioninViewport _returnvalue "(X=640.000000,Y=850.000000)" false)
        (UserInterface|Viewport|AddtoPlayerScreen _returnvalue)))
    (elif (and (>= _tempsreaction_2 2.7) (<= _tempsreaction_2 3.6))
      (Utilities|FlowControl|Sequence
        (:then_0
          (bind _asjeu_2 (Utilities|Casting|CastToJeu (Game|GetGameMode)))
          (Variables|/Game/Joueur/Jeu.Jeu_C|SetScore _asjeu_2 (+ (Variables|/Game/Joueur/Jeu.Jeu_C|GetScore _asjeu_2) 100))
          (bind _result_2 (Math|Integer|IncrementInt (Variables|/Game/Joueur/Jeu.Jeu_C|GetCombo _asjeu_2))
            (:%20%20
              (Variables|/Game/Joueur/Jeu.Jeu_C|SetCombo _asjeu_2 _result_2))))
        (:then_1
          (bind _returnvalue_2 (UserInterface|CreateWidget "/Game/Interface/FeedbackBien.FeedbackBien_C"))
          (Class|UserWidget|SetDesiredSizeinViewport _returnvalue_2 "(X=210.000000,Y=120.000000)")
          (Class|UserWidget|SetPositioninViewport _returnvalue_2 "(X=640.000000,Y=850.000000)" false)
          (UserInterface|Viewport|AddtoPlayerScreen _returnvalue_2)))
      (else
        (Utilities|FlowControl|Sequence
          (:then_0
            (bind _asjeu_3 (Utilities|Casting|CastToJeu (Game|GetGameMode)))
            (Variables|/Game/Joueur/Jeu.Jeu_C|SetScore _asjeu_3 (+ (Variables|/Game/Joueur/Jeu.Jeu_C|GetScore _asjeu_3) 50))
            (Variables|/Game/Joueur/Jeu.Jeu_C|SetCombo _asjeu_3 0))
          (:then_1
            (bind _returnvalue_3 (UserInterface|CreateWidget "/Game/Interface/FeedbackBof.FeedbackBof_C"))
            (Class|UserWidget|SetDesiredSizeinViewport _returnvalue_3 "(X=210.000000,Y=120.000000)")
            (Class|UserWidget|SetPositioninViewport _returnvalue_3 "(X=640.000000,Y=850.000000)" false)
            (UserInterface|Viewport|AddtoPlayerScreen _returnvalue_3))))))
  (bind _asjeu_4 (Utilities|Casting|CastToJeu (Game|GetGameMode)))
  (if (>= (Variables|/Game/Joueur/Jeu.Jeu_C|GetCombo _asjeu_4) 5)
    (Variables|/Game/Joueur/Jeu.Jeu_C|SetScore _asjeu_4 (+ (Variables|/Game/Joueur/Jeu.Jeu_C|GetScore _asjeu_4) (/ (Variables|/Game/Joueur/Jeu.Jeu_C|GetScore _asjeu_4) (Variables|/Game/Joueur/Jeu.Jeu_C|GetCombo _asjeu_4))))))